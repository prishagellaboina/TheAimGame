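; BP_Target is a target actor that can be switched between a visible active state and a hidden empty state.
; Tick polls the Active flag: when true it removes the first tag, shows the Sphere and clears the flag after a short Delay.
; When inactive, it hides the Sphere and sets its tags to EmptyTarget.
; A separate DestroyTarget function destroys the actor.
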(event `self.ReceiveBeginPlay`
  ;[1 1 1] Destroy Target if Not Hit
)

(event `self.ReceiveTick`
  (params (DeltaSeconds :type "Float (single-precision)"))
  (if (`self.Active`)
    (`KismetArrayLibrary.Array_Remove` (`self.Tags`))
    (`SceneComponent.SetHiddenInGame` (`self.Sphere`) false false)
    (`KismetSystemLibrary.Delay` 3.0)
    (set `self.Active` false)
    (else
      (`SceneComponent.SetHiddenInGame` (`self.Sphere`) true false)
      (set `self.Tags` (`|MakeArray` "EmptyTarget" :!type "Name")))))

(fn `DestroyTarget`
  (`self.K2_DestroyActor`))

(fn `UserConstructionScript`)
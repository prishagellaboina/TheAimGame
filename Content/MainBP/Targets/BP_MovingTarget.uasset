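; Shooting target that slides back and forth along Y and reports bullet hits to the gun.
; On BeginPlay, if the start object's LevelPlaying is already set, two chained timelines loop it between its spawn location and EndYPos.
; While LevelPlaying is true, head and body collision overlaps destroy the bullet, play a hit sound and call Headshot or Bodyshot on BP_Gun.
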(event `self.ReceiveBeginPlay`
  (bind (_returnvalue_x _returnvalue_y _returnvalue_z) (`KismetMathLibrary.BreakVector` (`self.K2_GetActorLocation`)))
  ;[1 1 1] Setting Start/End Pos and Gun Ref
  (set `self.Start` (`KismetMathLibrary.MakeVector` _returnvalue_x _returnvalue_y _returnvalue_z))
  (set `self.End` (`KismetMathLibrary.MakeVector` _returnvalue_x (`self.EndYPos`) _returnvalue_z))
  (bind _outactors (`GameplayStatics.GetAllActorsOfClass` "/Game/MainBP/BP_Gun.BP_Gun_C"))
  (set `self.Gun Ref` (`|GetArrayItem` _outactors))
  (bind _outactors_2 (`GameplayStatics.GetAllActorsOfClass` "/Game/MainBP/Targets/BP_MovingTargetsStart.BP_MovingTargetsStart_C"))
  (bind _output_get (set `self.StartObjRef` (`|GetArrayItem` _outactors_2)))
  (if (`/Game/MainBP/Targets/BP_MovingTargetsStart.LevelPlaying` _output_get)
    ;[1 1 1] Loop to Move Back and Forth
    (bind (_direction _movetrack) (`Timeline|MoveTo` :!via `PlayFromStart` :!label _label)
      (:`Update`
        (`self.K2_SetActorRelativeLocation` (`KismetMathLibrary.VLerp` (`self.Start`) (`self.End`) _movetrack)))
      (:`Finished`
        (bind (_direction_2 _movetrack_2) (`Timeline|MoveBack` :!via `ReverseFromEnd`)
          (:`Update`
            (`self.K2_SetActorRelativeLocation` (`KismetMathLibrary.VLerp` (`self.Start`) (`self.End`) _movetrack_2)))
          (:`Finished`
            (goto _label :!via `PlayFromStart`)))))))

(event `self.HeadCollision.OnComponentBeginOverlap`
  (params (OverlappedComponent :type "PrimitiveComponent Object Reference") (OtherActor :type "Actor Object Reference") (OtherComp :type "PrimitiveComponent Object Reference") (OtherBodyIndex :type Integer) (bFromSweep :type Boolean) (SweepResult :type "HitResult Structure (by ref)"))
  ;[1 1 1] Headshot
  (if (`/Game/MainBP/Targets/BP_MovingTargetsStart.LevelPlaying` (`self.StartObjRef`))
    (bind _asbp_bullet_projectile (cast `/Game/MainBP/BP_BulletProjectile` OtherActor))
    (`self.K2_DestroyActor` _asbp_bullet_projectile)
    (`GameplayStatics.PlaySoundAtLocation` "/Game/Assets/Sounds/Sound_TargetHit.Sound_TargetHit" (`self.K2_GetActorLocation`) (struct) 1.0 1.0 0.0 null null null)
    (`/Game/MainBP/BP_Gun.Headshot` (`self.Gun Ref`))))

(event `self.BodyCollision.OnComponentBeginOverlap`
  (params (OverlappedComponent :type "PrimitiveComponent Object Reference") (OtherActor :type "Actor Object Reference") (OtherComp :type "PrimitiveComponent Object Reference") (OtherBodyIndex :type Integer) (bFromSweep :type Boolean) (SweepResult :type "HitResult Structure (by ref)"))
  ;[1 1 1] Bodyshot
  (if (`/Game/MainBP/Targets/BP_MovingTargetsStart.LevelPlaying` (`self.StartObjRef`))
    (bind _asbp_bullet_projectile (cast `/Game/MainBP/BP_BulletProjectile` OtherActor))
    (`self.K2_DestroyActor` _asbp_bullet_projectile)
    (`GameplayStatics.PlaySoundAtLocation` "/Game/Assets/Sounds/Sound_Bodyshot.Sound_Bodyshot" (`self.K2_GetActorLocation`) (struct) 1.0 1.0 0.0 null null null)
    (`/Game/MainBP/BP_Gun.Bodyshot` (`self.Gun Ref`))))

(fn `UserConstructionScript`)
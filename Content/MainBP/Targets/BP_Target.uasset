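; BP_Target is a shooting target that shows for about three seconds while Active, then hides unless it is hit sooner.
; Tick polls Active to toggle sphere visibility and collision, using a Delay for the timeout and an "EmptyTarget" tag to mark inactive targets.
; An overlapping BP_BulletProjectile deactivates the target, is destroyed, reports the hit to the first BP_Gun found at BeginPlay, and plays a hit sound.
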(event `self.ReceiveTick`
  (params (DeltaSeconds :type "Float (single-precision)"))
  ;[1 1 1] Showing/Hiding Target Depending on State
  (if (`self.Active`)
    (`KismetArrayLibrary.Array_Remove` (`self.Tags`))
    (`SceneComponent.SetHiddenInGame` (`self.Sphere`) false false)
    (`self.SetActorEnableCollision` true)
    ;[1 1 1] Removing Target if Not Hit
    (`KismetSystemLibrary.Delay` 3.0)
    (set `self.Active` false)
    (else
      (`self.DeactivateTarget`))))

(event `self.ReceiveBeginPlay`
  (bind _outactors (`GameplayStatics.GetAllActorsOfClass` "/Game/MainBP/BP_Gun.BP_Gun_C"))
  (set `self.Gun` (`|GetArrayItem` _outactors)))

(event `self.CollisionSphere.OnComponentBeginOverlap`
  (params (OverlappedComponent :type "PrimitiveComponent Object Reference") (OtherActor :type "Actor Object Reference") (OtherComp :type "PrimitiveComponent Object Reference") (OtherBodyIndex :type Integer) (bFromSweep :type Boolean) (SweepResult :type "HitResult Structure (by ref)"))
  ;[1 1 1] On Bullet Collision
  ;;[1 1 1] Destroy Target and Bullet
  (bind _asbp_bullet_projectile (cast `/Game/MainBP/BP_BulletProjectile` OtherActor))
  (`self.DeactivateTarget`)
  (`self.K2_DestroyActor` _asbp_bullet_projectile)
  ;;[1 1 1] Update TargetsHit Variable
  (`/Game/MainBP/BP_Gun.OnTargetHit` (`self.Gun`))
  ;;[1 1 1] Play Sound Effect
  (`GameplayStatics.SpawnSoundAtLocation` "/Game/Assets/Sounds/Sound_TargetHit.Sound_TargetHit" (`SceneComponent.K2_GetComponentLocation` (`self.Sphere`)) (struct) 1.0 1.0 0.0 null null))

(fn `DeactivateTarget`
  (`SceneComponent.SetHiddenInGame` (`self.Sphere`) true false)
  (`self.SetActorEnableCollision` false)
  (set `self.Tags` (`|MakeArray` "EmptyTarget" :!type "Name"))
  (set `self.Active` false))

(fn `UserConstructionScript`)
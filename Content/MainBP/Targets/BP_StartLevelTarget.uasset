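; BP_StartLevelTarget is a shootable target that starts a timed level and handles its end.
; A bullet overlap hides the target, disables its collision and reveals the Timer-tagged UI.
; While playing, Tick drives a minutes/seconds countdown, throttled to one-second steps by a Delay.
; At zero, it plays a completion sound, calculates accuracy from BP_Gun's hit and shot counts, and reveals the end screen with collision enabled.
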(event `self.Box.OnComponentBeginOverlap`
  (params (OverlappedComponent :type "PrimitiveComponent Object Reference") (OtherActor :type "Actor Object Reference") (OtherComp :type "PrimitiveComponent Object Reference") (OtherBodyIndex :type Integer) (bFromSweep :type Boolean) (SweepResult :type "HitResult Structure (by ref)"))
  ;[1 1 1] Hide on Shoot and Start Level
  (cast `/Game/MainBP/BP_BulletProjectile` OtherActor)
  (set `self.LevelPlaying` true)
  (`SceneComponent.SetHiddenInGame` (`self.Cube`) true false)
  (`SceneComponent.SetHiddenInGame` (`self.Shoot To Start Text`) true false)
  (`self.SetActorEnableCollision` false)
  (bind _outactors (`GameplayStatics.GetAllActorsOfClassWithTag` "/Game/MainBP/UI/UIActor.UIActor_C" "Timer"))
  (`SceneComponent.SetHiddenInGame` (`/Game/MainBP/UI/UIActor.Widget` (`|GetArrayItem` _outactors)) false false))

(event `LevelEnd`
  (bind _gun_ref (`self.Gun Ref`))
  ;[1 1 1] Level End
  (`|ExecutionSequence`
    (:`then_0`
      ;;[1 1 1] Pause level, Set Gun Ref and Play Sound
      (set `self.LevelPlaying` false)
      (bind _outactors (`GameplayStatics.GetAllActorsOfClass` "/Game/MainBP/BP_Gun.BP_Gun_C"))
      (bind _output (`|GetArrayItem` _outactors))
      (set `self.Gun Ref` _output)
      (`GameplayStatics.PlaySoundAtLocation` "/Game/Assets/Sounds/Sound_Complete.Sound_Complete" (`self.K2_GetActorLocation` _output) (struct) 1.0 1.0 0.0 null null null))
    (:`then_1`
      ;;[1 1 1] Calculate Accuracy
      (set `self.Accuracy` (`KismetMathLibrary.FTrunc` (* (/ (`KismetMathLibrary.Conv_IntToDouble` (`/Game/MainBP/BP_Gun.TargetsHit` _gun_ref)) (`KismetMathLibrary.Conv_IntToDouble` (`/Game/MainBP/BP_Gun.AmmoFired` _gun_ref))) 100.0)))
      ;;[1 1 1] Enable End Screen and Collisions
      (bind _outactors_2 (`GameplayStatics.GetAllActorsOfClass` "/Game/MainBP/UI/EndScreenActor.EndScreenActor_C"))
      (bind _output_2 (`|GetArrayItem` _outactors_2))
      (`self.SetActorEnableCollision` _output_2 true)
      (`SceneComponent.SetHiddenInGame` (`/Game/MainBP/UI/EndScreenActor.Widget` _output_2) false false))))

(event `self.ReceiveTick`
  (params (DeltaSeconds :type "Float (single-precision)"))
  ;[1 1 1] Timer Countdown Tick
  (if (`self.LevelPlaying`)
    (`self.TimerCountdown`)))

(event `TimerCountdown`
  ;[1 1 1] Timer Countdown Tick
  (`KismetSystemLibrary.Delay` 1.0)
  (if (== (`self.Seconds`) 0)
    (if (== (`self.Minutes`) 0)
      (`self.LevelEnd`)
      (else
        (set `self.Seconds` 59)
        (set `self.Minutes` (- (`self.Minutes`) 1))))
    (else
      (set `self.Seconds` (- (`self.Seconds`) 1)))))

(fn `UserConstructionScript`)
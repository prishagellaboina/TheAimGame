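; VR gun actor, named for the menu, that a motion controller can pick up, drop and fire.
; Pickup disables physics and snaps the gun to the controller at a fixed offset, while Drop detaches it and restores physics.
; Trigger press spawns a scaled-down BP_BulletProjectile at a muzzle scene component, gated by CanFire until release, and plays a gunshot sound.
; GunGrabbed and FiredGun record first use and are never cleared here.
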(event `/Game/VirtualRealityBP/Blueprints/PickupActorInterface.Pickup`
  (params (AttachTo :type "SceneComponent Object Reference"))
  ;[1 1 1] Pickup and Drop Gun
  (`PrimitiveComponent.SetSimulatePhysics` (`self.StaticMeshComponent`) false)
  (`SceneComponent.K2_AttachToComponent` (`self.K2_GetRootComponent`) AttachTo "None" "SnapToTarget" "SnapToTarget" "KeepWorld" false)
  (`SceneComponent.K2_SetRelativeLocationAndRotation` (`self.StaticMeshComponent`) (-3.0 -1.0 0.0) (struct :`Yaw` -90.0 :`Roll` 10.0) false false)
  (set `self.GunGrabbed` true))

(event `/Game/VirtualRealityBP/Blueprints/PickupActorInterface.Drop`
  ;[1 1 1] Pickup and Drop Gun
  (`PrimitiveComponent.SetSimulatePhysics` (`self.StaticMeshComponent`) true)
  (`self.K2_DetachFromActor` "KeepWorld" "KeepWorld" "KeepWorld"))

(event `/Game/VirtualRealityBP/Blueprints/PickupActorInterface.TriggerPressed`
  ;[1 1 1] Trigger to Fire Bullets
  (`self.FireBullet`)
  ;[1 1 1] Play Gunshot Sound
  (`GameplayStatics.SpawnSoundAtLocation` "/Game/Assets/Sounds/Sound_Gunshot.Sound_Gunshot" (`SceneComponent.K2_GetComponentLocation` (`self.StaticMeshComponent`)) (struct) 1.0 1.0 0.0 null null)
  (set `self.FiredGun` true))

(event `/Game/VirtualRealityBP/Blueprints/PickupActorInterface.TriggerReleased`
  ;[1 1 1] Trigger to Fire Bullets
  (`self.ReleaseFireBullet`))

(fn `FireBullet`
  (bind (_returnvalue_location _returnvalue_rotation) (`KismetMathLibrary.BreakTransform` (`SceneComponent.K2_GetComponentToWorld` (`self.Scene`))))
  (if (`self.CanFire`)
    (`|SpawnActorFromClass` "/Game/MainBP/BP_BulletProjectile.BP_BulletProjectile_C" (`KismetMathLibrary.MakeTransform` _returnvalue_location _returnvalue_rotation (0.1 0.1 0.1)) "AlwaysSpawn" "OverrideRootScale" null null)
    (set `self.CanFire` false)))

(fn `ReleaseFireBullet`
  (set `self.CanFire` true))

(fn `UserConstructionScript`)